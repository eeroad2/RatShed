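; BP_RatProjectile is a rat projectile that either knocks the player back or becomes a spawned rat on impact.
; Its Box overlap ignores BP_Ratapult, then checks distance to player 0 rather than which actor it hit.
; A nearby player gets a clamped velocity-change impulse away from it, with a debug print; otherwise its Spawner spawns a child rat there.
; Either outcome spawns confetti and destroys the projectile.
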(event OnComponentBeginOverlap(Box)
  (params (OverlappedComponent :type Primitive%20Component%20Object%20Reference) (OtherActor :type Actor%20Object%20Reference) (OtherComp :type Primitive%20Component%20Object%20Reference) (OtherBodyIndex :type Integer) (bFromSweep :type Boolean) (SweepResult :type Hit%20Result%20Structure%20%28by%20ref%29))
  (bind _returnvalue (Game|GetPlayerCharacter 0))
  (bind _returnvalue_2 (Transformation|GetActorLocation))
  (bind _returnvalue_3 (Transformation|GetActorLocation _returnvalue))
  (bind _returnvalue_4 (- _returnvalue_3 _returnvalue_2))
  (bind _returnvalue_5 (* _returnvalue_4 3e+01))
  (Utilities|Casting|CastToBP_Ratapult OtherActor
    (:CastFailed
      (if (< (Transformation|GetDistanceTo _returnvalue) 6e+01)
        (Physics|AddImpulse (Variables|/Script/Engine.Character|GetCharacterMovement _returnvalue) (Math|Vector|ClampVectorSize _returnvalue_5 0.0 1.2e+03) true)
        (Development|PrintString (Utilities|String|ToString(Vector) _returnvalue_5))
        (else
          (Default|SpawnChildRat (Variables|Default|GetSpawner) _returnvalue_2)))
      (Niagara|SpawnSystematLocation "/Game/physical_layout/Confetti.Confetti" _returnvalue_2 "0, 0, 0" "0.500000,0.500000,0.500000")
      (Actor|DestroyActor))))

(event OnComponentHit(RatStaticMesh)
  (params (HitComponent :type Primitive%20Component%20Object%20Reference) (OtherActor :type Actor%20Object%20Reference) (OtherComp :type Primitive%20Component%20Object%20Reference) (NormalImpulse :type Vector :default "0, 0, 0") (Hit :type Hit%20Result%20Structure%20%28by%20ref%29)))

(event EventBeginPlay)

(event Collision|EventActorBeginOverlap
  (params (OtherActor :type Actor%20Object%20Reference)))

(event EventTick
  (params (DeltaSeconds :type Float%20%28single-precision%29)))

(fn ConstructionScript)