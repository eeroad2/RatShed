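; BP_Rat is an AI-controlled rat that holds a patrol path, a cheese reference and a damage value.
; On BeginPlay it finds its waypoint path and the first cheese, then enables movement through a Blackboard key.
; Patrol route changes cycle through level paths, writing PathIndex to the Blackboard only when wrapping to the first.
; StopMovement disables movement, then after a delay notifies the parent spawner, spawns confetti and destroys the rat.
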(event Custom|StopMovement
  (bind (_blackboard _name) (CallFunction|BBData "CanMove"))
  (Class|BlackboardComponent|SetValueasInt _blackboard _name)
  (Development|PrintString "Movement Stopped!")
  (Utilities|FlowControl|Delay 5.0)
  (CallFunction|Kill))

(event EventBeginPlay
  (bind (_blackboard _name) (CallFunction|BBData "CanMove"))
  (bind _outactors (Actor|GetAllActorsOfClass "/Game/Blueprints/BP_Waypoint_Path.BP_Waypoint_Path_C"))
  (Variables|Default|SetPatrolPath (Utilities|Array|Get(acopy) _outactors (Variables|Default|GetCurrentPatrolRoute)))
  (bind _outactors_2 (Actor|GetAllActorsOfClass "/Game/Blueprints/BP_Cheese.BP_Cheese_C"))
  (Variables|Default|SetCheese (Utilities|Array|Get(acopy) _outactors_2))
  (Class|BlackboardComponent|SetValueasInt _blackboard _name 1))

(event Collision|EventActorBeginOverlap
  (params (OtherActor :type Actor%20Object%20Reference)))

(event EventTick
  (params (DeltaSeconds :type Float%20%28single-precision%29)))

(event EventSetIndex
  (params (Index :type Integer))
  (Variables|Default|SetIndex Index))

(event EventSetPathIndex
  (params (NewIndex :type Integer))
  (bind (_blackboard _name) (CallFunction|BBData "PathIndex"))
  (bind _outactors (Actor|GetAllActorsOfClass "/Game/Blueprints/BP_Waypoint_Path.BP_Waypoint_Path_C"))
  (if (< NewIndex 0)
    (bind _output_get (Variables|Default|SetCurrentPatrolRoute (- (Utilities|Array|Length _outactors) 1)))
    (Variables|Default|SetPatrolPath (Utilities|Array|Get(acopy) _outactors _output_get))
    (elif (> NewIndex (- (Utilities|Array|Length _outactors) 1))
      (bind _output_get_2 (Variables|Default|SetCurrentPatrolRoute 0))
      (Variables|Default|SetPatrolPath (Utilities|Array|Get(acopy) _outactors _output_get_2))
      (Class|BlackboardComponent|SetValueasInt _blackboard _name (Variables|Default|GetCurrentPatrolRoute))
      (else
        (bind _output_get_3 (Variables|Default|SetCurrentPatrolRoute NewIndex))
        (Variables|Default|SetPatrolPath (Utilities|Array|Get(acopy) _outactors _output_get_3))))))

(fn ConstructionScript)

(fn BBData
  (params (KeyName :type Name))
  (return (AI|GetBlackboard (AI|GetAIController self)) (Utilities|Name|MakeLiteralName KeyName)))

(fn Kill
  (Default|RatDied (Variables|Default|GetParentSpawner) self)
  (Niagara|SpawnSystematLocation "/Game/physical_layout/Confetti.Confetti" (Transformation|GetActorLocation) "0, 0, 0" "0.750000,0.750000,0.750000")
  (Actor|DestroyActor))

(fn ChangePatrolPath
  (bind _pathindex (CallFunction|GetPathIndex))
  (CallFunction|SetPathIndex (+ _pathindex 1))
  (return (+ _pathindex 1)))

(fn GetCheese
  (return (Variables|Default|GetCheese)))

(fn GetDamage
  (return (Variables|Default|GetDamage)))

(fn GetIndex
  (return (Variables|Default|GetIndex)))

(fn GetPathIndex
  (return (Variables|Default|GetCurrentPatrolRoute)))

(fn GetPatrolPath
  (return (Variables|Default|GetPatrolPath)))