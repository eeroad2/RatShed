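; BP_Cheese is a damageable cheese actor that visibly loses pieces and whose depletion ends the game.
; TakeDamage lowers Health, destroying the first remaining static mesh component whenever the new value is a multiple of 20.
; If that new value is also negative, a DoOnce shows the game-over widget, switches input to UI with a cursor and blends the view to GameoverCamera.
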(event Custom|TakeDamage
  (params (Damage :type Integer))
  (bind _returnvalue (Game|GetPlayerController 0))
  (if (== (Math|Integer|%(Integer) (- (Variables|Default|GetHealth) Damage) 20) 0)
    (Components|DestroyComponent (Utilities|Array|Get(acopy) (Actor|GetComponentsByClass "/Script/Engine.StaticMeshComponent")))
    (if (< (- (Variables|Default|GetHealth) Damage) 0)
      (Utilities|FlowControl|DoOnce false
        (:Completed
          (bind _returnvalue_2 (UserInterface|CreateWidget "/Game/UI/gameover_bp.gameover_bp_C"))
          (UserInterface|Viewport|AddtoViewport _returnvalue_2 0)
          (Variables|/Script/Engine.PlayerController|SetbShowMouseCursor _returnvalue true)
          (Input|SetInputModeUIOnly _returnvalue _returnvalue_2 "DoNotLock" true)
          (Game|Player|SetViewTargetwithBlend (Game|GetPlayerController 0) (Utilities|ResolveSoftReference (Variables|Default|Getgameover_camera)) 0.0 "VTBlend_Linear" 0.0 false)))
      (else
        (Variables|Default|SetHealth (- (Variables|Default|GetHealth) Damage) :!label _label)))
    (else
      (goto _label))))

(event EventBeginPlay
  (Variables|Default|SetHealth 260)
  (Variables|Default|SetSegmentIndex 0))

(event Collision|EventActorBeginOverlap
  (params (OtherActor :type Actor%20Object%20Reference)))

(event EventTick
  (params (DeltaSeconds :type Float%20%28single-precision%29)))

(fn ConstructionScript)