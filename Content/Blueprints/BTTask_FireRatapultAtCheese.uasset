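; Behavior Tree task that makes an AI-controlled BP_Ratapult lob a rat projectile at its Cheese.
; It picks a random reachable point near the cheese and solves a custom-arc launch velocity from the ratapult's ProjectileLocation.
; It spawns BP_RatProjectile there, records the ratapult as Spawner, applies the velocity and finishes successfully.
; If the pawn is not a BP_Ratapult, the task never calls FinishExecute.
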(event EventReceiveExecuteAI
  (params (OwnerController :type AI%20Controller%20Object%20Reference) (ControlledPawn :type Pawn%20Object%20Reference))
  (bind _asbp_ratapult (Utilities|Casting|CastToBP_Ratapult ControlledPawn))
  (bind _outlaunchvelocity (Game|SuggestProjectileVelocityCustomArc (Transformation|GetWorldLocation (Variables|/Game/Blueprints/BP_Ratapult.BP_Ratapult_C|GetProjectileLocation _asbp_ratapult)) (.RandomLocation (AI|Navigation|GetRandomReachablePointinRadius (Transformation|GetActorLocation (Variables|/Game/Blueprints/BP_Ratapult.BP_Ratapult_C|GetCheese _asbp_ratapult)) 5e+01 0 0)) 0.0 0.5))
  (bind _returnvalue (Game|SpawnActorfromClass "/Game/Blueprints/BP_RatProjectile.BP_RatProjectile_C" (Math|Transform|MakeTransform (Transformation|GetWorldLocation (Variables|/Game/Blueprints/BP_Ratapult.BP_Ratapult_C|GetProjectileLocation _asbp_ratapult)) "0, 0, 0" "1.000000,1.000000,1.000000") "Undefined" "MultiplyWithRoot" 0 0))
  (Variables|/Game/Blueprints/BP_RatProjectile.BP_RatProjectile_C|SetSpawner _returnvalue _asbp_ratapult)
  (Game|Components|ProjectileMovement|SetVelocityinLocalSpace (Variables|/Game/Blueprints/BP_RatProjectile.BP_RatProjectile_C|GetProjectileMovement _returnvalue) _outlaunchvelocity)
  (AI|BehaviorTree|FinishExecute true))