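; BP_Ratapult is an AI-controlled enemy that spawns a capped number of child rats and takes several hits to destroy.
; Each tick it writes to its blackboard whether the player is near the cheese.
; SpawnChildRat links each new rat to itself and its parent spawner.
; Kill removes health, shaking the camera on non-fatal hits and, on death, notifying the spawner and playing confetti and a break sound before destroying itself.
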(event EventBeginPlay
  (bind _returnvalue (Actor|GetActorOfClass "/Game/Blueprints/BP_Cheese.BP_Cheese_C"))
  (Variables|Default|SetCheese _returnvalue)
  (Variables|Default|SetCurrentRats 0)
  (Variables|Default|SetMaxRats 5)
  (Variables|Default|SetHealth 3))

(event Collision|EventActorBeginOverlap
  (params (OtherActor :type Actor%20Object%20Reference)))

(event EventTick
  (params (DeltaSeconds :type Float%20%28single-precision%29))
  (AI|Components|Blackboard|SetValueasBool (AI|GetBlackboard (AI|GetAIController self)) (Utilities|Name|MakeLiteralName "PlayerAtCheese") (<= (Transformation|GetDistanceTo (Game|GetPlayerCharacter 0) (Variables|Default|GetCheese)) 1e+02)))

(fn ConstructionScript)

(fn SpawnChildRat
  (params (Location :type Vector))
  (if (< (Variables|Default|GetCurrentRats) (Variables|Default|GetMaxRats))
    (bind _returnvalue (Game|SpawnActorfromClass "/Game/Blueprints/BP_Rat.BP_Rat_C" (Math|Transform|MakeTransform Location "0, 0, 0" "1.000000,1.000000,1.000000") "Undefined" "MultiplyWithRoot" 0 0))
    (if (Utilities|IsValid _returnvalue)
      (Variables|/Game/Blueprints/BP_Rat.BP_Rat_C|SetParentSpawner _returnvalue (Variables|Default|GetParentSpawner))
      (Variables|/Game/Blueprints/BP_Rat.BP_Rat_C|SetRatapult _returnvalue self)
      (Variables|Default|SetCurrentRats (+ (Variables|Default|GetCurrentRats) 1)))))

(fn Kill
  (bind _returnvalue (Transformation|GetActorLocation))
  (Variables|Default|SetHealth (- (Variables|Default|GetHealth) 1))
  (if (<= (Variables|Default|GetHealth) 0)
    (Default|Ratapultdied (Variables|Default|GetParentSpawner) self)
    (Niagara|SpawnSystematLocation "/Game/physical_layout/Confetti.Confetti" _returnvalue "0, 0, 0" "0.750000,0.750000,0.750000")
    (Audio|PlaySoundatLocation "/Game/Blueprints/Lego_Break__Fall_Apart_-_Sound_Effect__HD_.Lego_Break__Fall_Apart_-_Sound_Effect__HD_" _returnvalue "0, 0, 0" 1.0 1.0 0.0 0 0 0 0)
    (Actor|DestroyActor)
    (else
      (Camera|PlayWorldCameraShake "/Game/Blueprints/RatapultKnock.RatapultKnock_C" (Transformation|GetActorLocation (Game|GetPlayerCharacter 0)) 0.0 1e+03))))