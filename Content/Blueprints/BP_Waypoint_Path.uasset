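; BP_Waypoint_Path is a spline-based waypoint path that hands out successive point locations to whatever follows it.
; GetNextSplinePosition steps a given index by the stored Direction and returns that spline point's world location and new index.
; At either end, a one-way path wraps to the opposite end, while other paths flip Direction to ping-pong.
; Direction lives on the path rather than being passed in by the caller.
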(event EventBeginPlay)

(event Collision|EventActorBeginOverlap
  (params (OtherActor :type Actor%20Object%20Reference)))

(event EventTick
  (params (DeltaSeconds :type Float%20%28single-precision%29)))

(fn ConstructionScript)

(fn GetNextSplinePosition
  (params (Index :type Integer))
  (bind _spline (Variables|Default|GetSpline))
  (bind _returnvalue (Spline|GetNumberOfSplinePoints _spline))
  (bind _returnvalue_2 (- _returnvalue 1))
  ;[0.15 0.15 0.15 0.5] Check if next index is out of bounds
  (if (or (< (+ Index (Variables|Default|GetDirection)) 0) (> (+ Index (Variables|Default|GetDirection)) _returnvalue_2))
    ;[0.15 0.15 0.15 0.5] If so, check if path is one way
    (if (Variables|Default|GetIsOneWay)
      ;[0.15 0.15 0.15 0.5] if so, check if next index is -1
      (if (< (+ Index (Variables|Default|GetDirection)) 0)
        ;[0.15 0.15 0.15 0.5] if so, set next index to the endpoint
        (Variables|Default|SetIndex _returnvalue_2)
        (else
          ;[0.15 0.15 0.15 0.5] if not, then the next index is greater than tthe max, so set the iindex to 0
          (Variables|Default|SetIndex 0)))
      (else
        ;[0.15 0.15 0.15 0.5] if not, switch directions
        (Variables|Default|SetDirection (* (Variables|Default|GetDirection) -1))
        ;[0.15 0.15 0.15 0.5] If not, increment index in current direction
        (Variables|Default|SetIndex (+ (Variables|Default|GetDirection) Index) :!label _label)))
    (else
      (goto _label)))
  (return (Spline|GetLocationatSplinePoint _spline Index "World") (Variables|Default|GetIndex)))